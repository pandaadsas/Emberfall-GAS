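; GA_FireBolt is a gameplay ability that casts fire bolt projectiles at the target under the mouse.
; After committing, it takes the hit actor and location from target data, turns the avatar toward that point and plays the cast montage.
; A montage gameplay event spawns the projectiles from the weapon socket with an overridden launch pitch, homing on the hit actor.
; The ability ends when the montage completes, blends out, is interrupted or is cancelled.
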(event Ability|EventActivateAbility
  (bind _returnvalue (Ability|CommitAbility))
  (if _returnvalue
    (bind _datahandle (|TargetDataUnderMouse)
      (:ValidData
        (Variables|Default|SetHit%20Actor (.HitActor (Collision|BreakHitResult (Ability|TargetData|GetHitResultfromTargetData _datahandle))))
        (Variables|Default|SetProjectileTargetLocation (.Location (Collision|BreakHitResult (Ability|TargetData|GetHitResultfromTargetData _datahandle))))
        (Class|CombatInterface|UpdateFacingTarget(Message) (Ability|GetAvatarActorfromActorInfo) (Variables|Default|GetProjectileTargetLocation))
        (|PlayMontageandWaitProxy "None" "/Game/Assets/Characters/Aura/Animations/Abilities/AM_Cast_FireBolt.AM_Cast_FireBolt" 1.0 "None" false 1.0 0.0 false
          (:then
            (Ability|Tasks|WaitGameplayEvent "(TagName=\"Event.Montage.FireBolt\")" 0 true
              (:EventReceived
                (Class|DuraFireBolt|SpawnProjectiles (Variables|Default|GetProjectileTargetLocation) (GameplayTags|MakeLiteralGameplayTag "(TagName=\"CombatSocket.Weapon\")") true 45.0 (Variables|Default|GetHit%20Actor)))))
          (:OnCompleted
            (Ability|EndAbility :!label _label))
          (:OnBlendOut
            (goto _label))
          (:OnInterrupted
            (goto _label))
          (:OnCancelled
            (goto _label)))))))